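; BP_DrawblePlane is a drawable surface, set up for multiplayer, that players can paint on with textured brushes.
; On BeginPlay or clear, it creates a white render target, shows it through a dynamic material on the plane, and creates a brush material instance.
; Server and multicast draw events stamp that brush onto the render target at a normalized location.
; OnRep handlers reapply brush texture and plane material, and another event copies the material to a second plane.
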(event `Server_Set Mat`
  (params (Material :type "MaterialInterface Object Reference"))
  (`PrimitiveComponent.SetMaterial` (`self.Plane`) 0 Material))

(event `Multi_Set second plane`
  (`PrimitiveComponent.SetMaterial` (`/Game/Blueprints/Enviroment/BP_DrawblePlane.Plane` (`self.SecondPlane`)) 0 (`PrimitiveComponent.GetMaterial` (`self.Plane`) 0)))

(event `Multi_ClearPlane`
  (`self.Clear Plane`))

(event `Multicast_DrawBrush`
  (params (BrushTexture :type "Texture2D Object Reference") (BrushSize :type "Float (double-precision)") (DrawLocation :type "Vector2D Structure"))
  (`|ExecutionSequence`
    (:`then_0`
      (bind _output_get (set `self.BrushTextue` BrushTexture))
      (`MaterialInstanceDynamic.SetTextureParameterValue` (`self.BrushMaterial`) "BrushTexture" _output_get))
    (:`then_1`
      (bind (_canvas _size _context) (`KismetRenderingLibrary.BeginDrawCanvasToRenderTarget` (`self.RenderTarget`)))
      (`Canvas.K2_DrawMaterial` _canvas (`self.BrushMaterial`) (- (* _size DrawLocation) (/ BrushSize 0.0)) (`KismetMathLibrary.MakeVector2D` BrushSize BrushSize) (0.0 0.0) (1.0 1.0) 0.0 (0.5 0.5))
      (`KismetRenderingLibrary.EndDrawCanvasToRenderTarget` _context)
      (set `self.New Mat` (`PrimitiveComponent.GetMaterial` (`self.Plane`) 0)))))

(event `Server_DrawBrush`
  (params (BrushTexture :type "Texture2D Object Reference") (BrushSize :type "Float (double-precision)") (DrawLocation :type "Vector2D Structure"))
  (`|ExecutionSequence`
    (:`then_0`
      (bind _output_get (set `self.BrushTextue` BrushTexture))
      (`MaterialInstanceDynamic.SetTextureParameterValue` (`self.BrushMaterial`) "BrushTexture" _output_get))
    (:`then_1`
      (bind (_canvas _size _context) (`KismetRenderingLibrary.BeginDrawCanvasToRenderTarget` (`self.RenderTarget`)))
      (`Canvas.K2_DrawMaterial` _canvas (`self.BrushMaterial`) (- (* _size DrawLocation) (/ BrushSize 0.0)) (`KismetMathLibrary.MakeVector2D` BrushSize BrushSize) (0.0 0.0) (1.0 1.0) 0.0 (0.5 0.5))
      (`KismetRenderingLibrary.EndDrawCanvasToRenderTarget` _context))))

(event `Clear Plane`
  (`|ExecutionSequence` :!label _label
    (:`then_0`
      (bind _returnvalue (`KismetRenderingLibrary.CreateRenderTarget2D` 1024 1024))
      (bind _output_get (set `self.RenderTarget` _returnvalue))
      (`KismetRenderingLibrary.ClearRenderTarget2D` _output_get (struct :`R` 1.0 :`G` 1.0 :`B` 1.0 :`A` 1.0)))
    (:`then_1`
      (bind _returnvalue_2 (`KismetMaterialLibrary.CreateDynamicMaterialInstance` "/Game/Art/Materials/M_DrawingMaterial.M_DrawingMaterial"))
      (`MaterialInstanceDynamic.SetTextureParameterValue` _returnvalue_2 "RenderTarget" (`self.RenderTarget`))
      (`PrimitiveComponent.SetMaterial` (`self.Plane`) 0 _returnvalue_2))
    (:`then_2`
      (bind _returnvalue_3 (`KismetMaterialLibrary.CreateDynamicMaterialInstance` "/Game/Art/Materials/M_BrashMat.M_BrashMat"))
      (set `self.BrushMaterial` _returnvalue_3))))

(event `self.ReceiveBeginPlay`
  (goto _label))

(fn `OnRep_BrushTextue`
  (`MaterialInstanceDynamic.SetTextureParameterValue` (`self.BrushMaterial`) "BrushTexture" (`self.BrushTextue`)))

(fn `OnRep_New Mat`
  (`self.Server_Set Mat` (`self.New Mat`)))

(fn `OnRep_RenderTarget`)

(fn `UserConstructionScript`)